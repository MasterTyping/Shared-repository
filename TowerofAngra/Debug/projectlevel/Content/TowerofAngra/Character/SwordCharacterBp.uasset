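; Sword character Blueprint that conjures a magic circle at its shield when the Skill input is pressed.
; The press spawns a Magic_CircleBP at the mesh's "shield" socket transform, with the roll offset by 90 degrees, and stores the reference.
; Tick moves the stored circle to the socket's location while it is valid, without updating rotation.
; Each press overwrites the reference without destroying the previous circle, so only the newest follows.
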(event `self.ReceiveTick`
  (params (DeltaSeconds :type "Float (single-precision)"))
  (`/Engine/EditorBlueprintResources/StandardMacros.IsValid` (stale `InputAction|Skill` _returnvalue)
    (:`Is Valid`
      (`self.K2_SetActorLocation` (stale `InputAction|Skill` _returnvalue) (.location (`SceneComponent.GetSocketTransform` (`self.Mesh`) "shield" "RTS_World")) false false))))

(event `InputAction|Skill`
  (params (Key :type "Key Structure"))
  (:`Pressed`
    (bind _returnvalue (`|SpawnActorFromClass` "/Game/TowerofAngra/Effect/Magic_Circle/Magic_CircleBP.Magic_CircleBP_C" (`KismetMathLibrary.MakeTransform` (.location (`SceneComponent.GetSocketTransform` (`self.Mesh`) "shield" "RTS_World")) (`KismetMathLibrary.MakeRotator` (+ (.roll (.rotation (`SceneComponent.GetSocketTransform` (`self.Mesh`) "shield" "RTS_World"))) 90.0) (.pitch (.rotation (`SceneComponent.GetSocketTransform` (`self.Mesh`) "shield" "RTS_World"))) (.yaw (.rotation (`SceneComponent.GetSocketTransform` (`self.Mesh`) "shield" "RTS_World")))) (.scale (`SceneComponent.GetSocketTransform` (`self.Mesh`) "shield" "RTS_World"))) "Undefined" "OverrideRootScale" null null))))

(fn `UserConstructionScript`)