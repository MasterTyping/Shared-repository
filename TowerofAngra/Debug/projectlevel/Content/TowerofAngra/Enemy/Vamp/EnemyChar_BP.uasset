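; EnemyChar_BP is an enemy character with walk and run speeds, a melee attack and a death response.
; Attack plays a downward swing and holds an Attacking flag for a fixed delay before restoring the Animation Blueprint.
; Capsule overlaps during that window damage player 0's MagicianCharacter, without checking which actor overlapped.
; Died plays a dying animation and clears the AI controller class.
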(event `self.ReceiveBeginPlay`)

(event `Walk`
  (set `CharacterMovementComponent.MaxWalkSpeed` 200.0 (`self.CharacterMovement`)))

(event `run`
  (set `CharacterMovementComponent.MaxWalkSpeed` 400.0 (`self.CharacterMovement`)))

(event `Attack`
  (`SkeletalMeshComponent.PlayAnimation` (`self.Mesh`) "/Game/TowerofAngra/Enemy/Vamp/Anim/Standing_Melee_Attack_Downward.Standing_Melee_Attack_Downward" false)
  (set `self.Attacking` true)
  (`KismetSystemLibrary.Delay` 2.67)
  (set `self.Attacking` false)
  (`SkeletalMeshComponent.SetAnimationMode` (`self.Mesh`) "AnimationBlueprint"))

(event `self.ReceiveTick`
  (params (DeltaSeconds :type "Float (single-precision)")))

(event `Died`
  (`SkeletalMeshComponent.PlayAnimation` (`self.Mesh`) "/Game/TowerofAngra/Enemy/Vamp/Anim/mutant_dying.mutant_dying" false)
  (set `self.AIControllerClass` null))

(event `self.Capsule.OnComponentBeginOverlap`
  (params (OverlappedComponent :type "PrimitiveComponent Object Reference") (OtherActor :type "Actor Object Reference") (OtherComp :type "PrimitiveComponent Object Reference") (OtherBodyIndex :type Integer) (bFromSweep :type Boolean) (SweepResult :type "HitResult Structure (by ref)"))
  (if (`self.Attacking`)
    (bind _asmagician_character (cast `/Game/TowerofAngra/Character/MagicianCharacter` (`GameplayStatics.GetPlayerCharacter` 0)))
    (`/Game/TowerofAngra/Character/MagicianCharacter.TakeDamage` _asmagician_character (`self.Damage`))))

(fn `UserConstructionScript`)